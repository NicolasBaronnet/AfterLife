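; Test character that moves along world axes from the MoveForward and MoveRight inputs and turns to face the input direction.
; Each Tick, GetDirectionAngle derives the signed angle between actor forward and the input vector using dot product arccosine and cross product Z sign.
; The actor rotates in fixed yaw steps, independent of delta time, outside a small tolerance.
; The angle prints for debugging; the computed planar speed drives nothing.
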(event EventBeginPlay)

(event Collision|EventActorBeginOverlap
  (params (OtherActor :type Actor%20Object%20Reference)))

(event EventTick
  (params (DeltaSeconds :type Float%20%28single-precision%29))
  (CallFunction|GetSpeed)
  (bind _output_get (Variables|Default|SetForwardRef (Math|Vector|MakeVector (Variables|Default|GetSideSpeed) (Variables|Default|GetForwardSpeed) 0.0)))
  (bind _returnvalue (CallFunction|GetDirectionAngle _output_get))
  (Development|PrintString (Utilities|String|ToString(Float) _returnvalue))
  (if (Math|Float|InRange(Float) _returnvalue 0.0 1.8e+02)
    (if (not (Math|Float|NearlyEqual(Float) _returnvalue 0.0 5.0))
      (Transformation|AddActorLocalRotation "0,7.000000, 0" false false))
    (elif (not (Math|Float|NearlyEqual(Float) _returnvalue 0.0 5.0))
      (Transformation|AddActorLocalRotation "0,-7.000000, 0" false false))))

(event Input|AxisEvents|InputAxisMoveForward
  (params (AxisValue :type Float%20%28single-precision%29))
  (bind _output_get (Variables|Default|SetForwardSpeed AxisValue))
  (Pawn|Input|AddMovementInput "0.000000,1.000000, 0" _output_get false))

(event Input|AxisEvents|InputAxisMoveRight
  (params (AxisValue :type Float%20%28single-precision%29))
  (bind _output_get (Variables|Default|SetSideSpeed AxisValue))
  (Pawn|Input|AddMovementInput "1.000000,0.000000, 0" _output_get false))

(fn ConstructionScript)

(fn GetSpeed
  (bind _self self)
  (bind _returnvalue (Transformation|GetVelocity _self))
  (bind _output_get (Variables|Default|SetActualSpeed (Math|Float|Sqrt (+ (Math|Float|Square (.x _returnvalue)) (Math|Float|Square (.y _returnvalue))))))
  (return _output_get))

(fn GetDirectionAngle
  (params (A :type Vector))
  (bind _returnvalue (Transformation|GetActorForwardVector))
  (bind _returnvalue_2 (Math|Vector|Normalize A))
  (bind _returnvalue_3 (Math|Vector|Normalize _returnvalue))
  (return (* (Class|KismetMathLibrary|DegAcos (Math|Vector|DotProduct _returnvalue_3 _returnvalue_2)) (Math|Float|Sign(Float) (.z (Math|Vector|CrossProduct _returnvalue_3 _returnvalue_2))))))