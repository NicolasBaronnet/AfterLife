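; Destructible cube obstacle that shatters when the hero or a stunned Starved Body rams it.
; Game mode dispatchers for charging, walking and axe hits set IsCharging, which Tick uses to switch the cube's Pawn collision between Overlap and Block.
; On overlap during a hero dash, parry or axe hit, or by a stunned body, it applies impulse damage, then disables physics simulation after a delay.
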(event OnComponentBeginOverlap(DM_Cube)
  (params (OverlappedComponent :type Primitive%20Component%20Object%20Reference) (OtherActor :type Actor%20Object%20Reference) (OtherComp :type Primitive%20Component%20Object%20Reference) (OtherBodyIndex :type Integer) (bFromSweep :type Boolean) (SweepResult :type Hit%20Result%20Structure%20%28by%20ref%29))
  (bind _dm_cube (Variables|Default|GetDM_Cube))
  (bind _dm_cube_2 (Variables|Default|GetDM_Cube))
  (bind _asbp_hero (Utilities|Casting|CastToBP_Hero OtherActor)
    (:then
      (if (Math|Boolean|ORBoolean (.InDash (Utilities|Struct|BreakS_States (Variables|/Game/Hero/BP_Hero.BP_Hero_C|GetCharacBehavior _asbp_hero))) (.InParry (Utilities|Struct|BreakS_States (Variables|/Game/Hero/BP_Hero.BP_Hero_C|GetCharacBehavior _asbp_hero))) (.InAxeHit (Utilities|Struct|BreakS_States (Variables|/Game/Hero/BP_Hero.BP_Hero_C|GetCharacBehavior _asbp_hero))))
        (Class|DestructibleComponent|ApplyDamage (Variables|Default|GetDM_Cube) 2.0 (.impactpoint SweepResult) (.normal SweepResult) 1e+04)
        (Utilities|FlowControl|Delay 5.0)
        (Physics|SetSimulatePhysics _dm_cube_2 false)
        (Collision|SetCollisionEnabled _dm_cube_2 "QueryAndPhysics")))
    (:CastFailed
      (bind _asbp_starved_body (Utilities|Casting|CastToBP_Starved_Body OtherActor))
      (if (.Stunned (Utilities|Struct|BreakS_StarvedBehavior (Variables|/Game/Enemies/Starved/BP_Starved_Body.BP_Starved_Body_C|GetS_StarvedBehavior _asbp_starved_body)))
        (Class|DestructibleComponent|ApplyDamage (Variables|Default|GetDM_Cube) 2.0 (.impactpoint SweepResult) (.normal SweepResult) 1e+04)
        (Utilities|FlowControl|Delay 5.0)
        (Physics|SetSimulatePhysics _dm_cube false)
        (Collision|SetCollisionEnabled _dm_cube "QueryAndPhysics")))))

(event Custom|Charging
  (Variables|Default|SetIsCharging? true))

(event Custom|Walking
  (Variables|Default|SetIsCharging? false))

(event Custom|EDAxeHit_Event_0
  (Variables|Default|SetIsCharging? true))

(event EventBeginPlay
  (bind _gamemodref (CallFunction|GetGameMod))
  (EventDispatchers|BindEventtoEDIsCharging? _gamemodref (delegate Custom|Charging))
  (EventDispatchers|BindEventtoEDWalking _gamemodref (delegate Custom|Walking))
  (EventDispatchers|AssignEDAxeHit _gamemodref (delegate Custom|EDAxeHit_Event_0)))

(event Collision|EventActorBeginOverlap
  (params (OtherActor :type Actor%20Object%20Reference)))

(event EventTick
  (params (DeltaSeconds :type Float%20%28single-precision%29))
  (Utilities|FlowControl|Sequence
    (:then_0
      (if (Variables|Default|GetIsCharging?)
        (Collision|SetCollisionResponsetoChannel (Variables|Default|GetDM_Cube) "ECC_Pawn" "ECR_Overlap")
        (else
          (Collision|SetCollisionResponsetoChannel (Variables|Default|GetDM_Cube) "ECC_Pawn" "ECR_Block"))))))

(fn ConstructionScript)