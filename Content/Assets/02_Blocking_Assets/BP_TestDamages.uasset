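; BP_TestDamages is a blocking-asset test volume that repeatedly damages the hero while it stands inside its Box.
; When a BP_Hero's capsule begins overlapping the Box, a one-second looping timer starts, calling ApplyDamages, which passes -10 to the hero's LifeGestureFunction.
; When the capsule ends overlap, the stored timer handle is cleared, stopping the damage.
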(event OnComponentBeginOverlap(Box)
  (params (OverlappedComponent :type Primitive%20Component%20Object%20Reference) (OtherActor :type Actor%20Object%20Reference) (OtherComp :type Primitive%20Component%20Object%20Reference) (OtherBodyIndex :type Integer) (bFromSweep :type Boolean) (SweepResult :type Hit%20Result%20Structure%20%28by%20ref%29))
  (bind _asbp_hero (Utilities|Casting|CastToBP_Hero OtherActor))
  (if (== OtherComp (Variables|/Script/Engine.Character|GetCapsuleComponent _asbp_hero))
    (bind _returnvalue (Utilities|Time|SetTimerbyEvent (delegate Custom|ApplyDamages) 1.0 true))
    (Variables|Default|SetDamageTimer _returnvalue)))

(event OnComponentEndOverlap(Box)
  (params (OverlappedComponent :type Primitive%20Component%20Object%20Reference) (OtherActor :type Actor%20Object%20Reference) (OtherComp :type Primitive%20Component%20Object%20Reference) (OtherBodyIndex :type Integer))
  (bind _asbp_hero (Utilities|Casting|CastToBP_Hero OtherActor))
  (if (== (Variables|/Script/Engine.Character|GetCapsuleComponent _asbp_hero) OtherComp)
    (Utilities|Time|ClearandInvalidateTimerbyHandle (Variables|Default|GetDamageTimer))))

(event Custom|ApplyDamages
  (Default|LifeGestureFunction (stale OnComponentBeginOverlap(Box) _asbp_hero) -10))

(event EventBeginPlay)

(event Collision|EventActorBeginOverlap
  (params (OtherActor :type Actor%20Object%20Reference)))

(event EventTick
  (params (DeltaSeconds :type Float%20%28single-precision%29)))

(fn ConstructionScript)