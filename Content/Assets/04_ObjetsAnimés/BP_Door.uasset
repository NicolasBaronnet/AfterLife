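; Vertically sliding gate actor that opens and closes through GoesUp and GoesDown events, with no trigger logic of its own.
; Each event toggles the Box collision (off to open, on to close), waits a delay, then starts a looping timer.
; The timer nudges Door in fixed Z steps until it reaches the Top or Bot marker, then clears itself.
; DoOnce gates play the open or close sound once per movement.
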(event Custom|GoesUpTimer
  ;[1 1 1] Timer Go Top
  (if (> (.z (Transformation|GetWorldLocation (Variables|Default|GetTop))) (.z (Transformation|GetWorldLocation (Variables|Default|GetDoor))))
    (Transformation|AddWorldOffset (Variables|Default|GetDoor) "0, 0,1.300000" false false)
    (Utilities|FlowControl|DoOnce false :!label _label
      (:Completed
        (Audio|PlaySoundatLocation "/Game/Sounds/Cue/Environnement/SC_Gate_Open.SC_Gate_Open" (Transformation|GetActorLocation self) "0, 0, 0" 1.0 1.0 0.0 0 0 0)))
    (else
      (Utilities|Time|ClearandInvalidateTimerbyHandle (Variables|Default|GetGoesUpTimerHandle))
      (goto _label Reset))))

(event Custom|GoesDown
  ;[1 1 1] Timer Go Down
  (Collision|SetCollisionEnabled (Variables|Default|GetBox) "QueryAndPhysics")
  (Utilities|FlowControl|Delay (Variables|Default|GetWaitDuration))
  (bind _returnvalue (Utilities|Time|SetTimerbyEvent (delegate Custom|GoesDownTimer) (Variables|Default|GetSpeed) true))
  (Variables|Default|SetGoesDownTimerHandle _returnvalue))

(event Custom|GoesUp
  ;[1 1 1] Timer Go Top
  (Collision|SetCollisionEnabled (Variables|Default|GetBox) "NoCollision")
  (Utilities|FlowControl|Delay (Variables|Default|GetWaitDuration))
  (bind _returnvalue (Utilities|Time|SetTimerbyEvent (delegate Custom|GoesUpTimer) (Variables|Default|GetSpeed) true))
  (Variables|Default|SetGoesUpTimerHandle _returnvalue))

(event Custom|GoesDownTimer
  ;[1 1 1] Timer Go Down
  (if (> (.z (Transformation|GetWorldLocation (Variables|Default|GetDoor))) (.z (Transformation|GetWorldLocation (Variables|Default|GetBot))))
    (Transformation|AddWorldOffset (Variables|Default|GetDoor) "0, 0,-1.300000" false false)
    (Utilities|FlowControl|DoOnce false :!label _label
      (:Completed
        (Audio|PlaySoundatLocation "/Game/Sounds/Cue/Environnement/SC_Gate_Close.SC_Gate_Close" (Transformation|GetActorLocation self) "0, 0, 0" 1.0 1.0 0.0 0 0 0)))
    (else
      (Utilities|Time|ClearandInvalidateTimerbyHandle (Variables|Default|GetGoesDownTimerHandle))
      (goto _label Reset))))

(event EventBeginPlay)

(event EventTick
  (params (DeltaSeconds :type Float%20%28single-precision%29)))

(fn ConstructionScript
  (Collision|SetCollisionEnabled (Variables|Default|GetBox) "NoCollision"))