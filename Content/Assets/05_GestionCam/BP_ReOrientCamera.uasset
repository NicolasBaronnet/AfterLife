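; Trigger volume that tilts the hero's camera when BP_Hero enters its box and copies its HandFalling value onto the hero.
; The overlap plays the RotateCamera timeline, which adds local pitch to the hero's SpringArm, scaled by CameraSpeed, with GoToBase choosing the direction.
; The timeline stops once the arm's pitch reaches either limit of its range, between steeply angled and straight down.
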(event OnComponentBeginOverlap(Box)
  (params (OverlappedComponent :type Primitive%20Component%20Object%20Reference) (OtherActor :type Actor%20Object%20Reference) (OtherComp :type Primitive%20Component%20Object%20Reference) (OtherBodyIndex :type Integer) (bFromSweep :type Boolean) (SweepResult :type Hit%20Result%20Structure%20%28by%20ref%29))
  (bind _asbp_hero (Utilities|Casting|CastToBP_Hero OtherActor))
  (Variables|/Game/Hero/BP_Hero.BP_Hero_C|SetHandFalling _asbp_hero (Variables|Default|GetHandFalling))
  (bind _newtrack_0 (Timeline|RotateCamera Play)
    (:Update
      (Utilities|FlowControl|Sequence
        (:then_0
          (if (Variables|Default|GetGoToBase?)
            (Transformation|AddLocalRotation (Variables|/Game/Hero/BP_Hero.BP_Hero_C|GetSpringArm _asbp_hero) (Math|Rotator|MakeRotator 0.0 (* (Variables|Default|GetCameraSpeed) _newtrack_0) 0.0) false false)
            (else
              (Transformation|AddLocalRotation (Variables|/Game/Hero/BP_Hero.BP_Hero_C|GetSpringArm _asbp_hero) (Math|Rotator|MakeRotator 0.0 (* _newtrack_0 (Variables|Default|GetCameraSpeed) -1.0) 0.0) false false))))
        (:then_1
          (if (or (<= (.pitch (Variables|/Script/Engine.SceneComponent|GetRelativeRotation (Variables|/Game/Hero/BP_Hero.BP_Hero_C|GetSpringArm _asbp_hero))) -9e+01) (>= (.pitch (Variables|/Script/Engine.SceneComponent|GetRelativeRotation (Variables|/Game/Hero/BP_Hero.BP_Hero_C|GetSpringArm _asbp_hero))) -6e+01))
            (Timeline|RotateCamera Stop)))))))

(event EventBeginPlay)

(event Collision|EventActorBeginOverlap
  (params (OtherActor :type Actor%20Object%20Reference)))

(event EventTick
  (params (DeltaSeconds :type Float%20%28single-precision%29)))

(fn ConstructionScript)