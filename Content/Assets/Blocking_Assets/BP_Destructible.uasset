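; Destructible cube obstacle that blocks pawns normally and breaks apart when overlapped during a charge.
; Game mode dispatchers for charging and axe hit set IsCharging, and the walking dispatcher clears it.
; Tick switches the cube's Pawn collision response between Overlap and Block from that flag.
; Any begin overlap on the cube applies heavy damage and an impulse using the sweep's impact point and normal.
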(event OnComponentBeginOverlap(DM_Cube)
  (params (OverlappedComponent :type Primitive%20Component%20Object%20Reference) (OtherActor :type Actor%20Object%20Reference) (OtherComp :type Primitive%20Component%20Object%20Reference) (OtherBodyIndex :type Integer) (bFromSweep :type Boolean) (SweepResult :type Hit%20Result%20Structure%20%28by%20ref%29))
  (Class|DestructibleComponent|ApplyDamage (Variables|Default|GetDM_Cube) 2e+02 (.impactpoint SweepResult) (.normal SweepResult) 2e+04))

(event Custom|Charging
  (Variables|Default|SetIsCharging? true))

(event Custom|Walking
  (Variables|Default|SetIsCharging? false))

(event Custom|EDAxeHit_Event_0
  (Variables|Default|SetIsCharging? true))

(event EventBeginPlay
  (bind _gamemodref (CallFunction|GetGameMod))
  (EventDispatchers|BindEventtoEDIsCharging? _gamemodref (delegate Custom|Charging))
  (EventDispatchers|BindEventtoEDWalking _gamemodref (delegate Custom|Walking))
  (EventDispatchers|AssignEDAxeHit _gamemodref (delegate Custom|EDAxeHit_Event_0)))

(event Collision|EventActorBeginOverlap
  (params (OtherActor :type Actor%20Object%20Reference)))

(event EventTick
  (params (DeltaSeconds :type Float%20%28single-precision%29))
  (Utilities|FlowControl|Sequence
    (:then_0
      (if (Variables|Default|GetIsCharging?)
        (Collision|SetCollisionResponsetoChannel (Variables|Default|GetDM_Cube) "ECC_Pawn" "ECR_Overlap")
        (else
          (Collision|SetCollisionResponsetoChannel (Variables|Default|GetDM_Cube) "ECC_Pawn" "ECR_Block"))))))

(fn ConstructionScript)