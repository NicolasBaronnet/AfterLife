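; BP_InteractiveObjectsParent is a base actor for interactive objects that shows a Halo effect while the mouse cursor hovers over it.
; Every Tick it line-traces under the cursor on Visibility and checks that this actor is hit and BP_Hero is not inspecting.
; Two DoOnce gates reset each other, so Halo activates or deactivates only when that hover state changes.
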(event EventBeginPlay)

(event Collision|EventActorBeginOverlap
  (params (OtherActor :type Actor%20Object%20Reference)))

(event EventTick
  (params (DeltaSeconds :type Float%20%28single-precision%29))
  ;[1 1 1] Spawn emmiter on mouseouver
  (bind _asbp_hero (Utilities|Casting|CastToBP_Hero (Game|Player|GetPlayerPawn 0)))
  (if (and (== (.hitactor (.HitResult (Game|Player|GetHitResultUnderCursorbyChannel (Game|GetPlayerController 0) "TraceTypeQuery1" true))) self) (not (Variables|/Game/Hero/BP_Hero.BP_Hero_C|GetIsInspecting _asbp_hero)))
    (Utilities|FlowControl|DoOnce false :!label _label
      (:Completed
        (Components|Activation|SetActive (Variables|Default|GetHalo) true false)
        (goto _label_2 Reset)))
    (else
      (Utilities|FlowControl|DoOnce false :!label _label_2
        (:Completed
          (Components|Activation|SetActive (Variables|Default|GetHalo) false false)
          (goto _label Reset))))))

(fn ConstructionScript)