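; BP_Pont is a bridge actor that collapses when the hero enters its trigger box.
; On overlap with BP_Hero, it damages its Destructible component at the actor's location, with the impulse directed along the hero's downward axis.
; It then switches the component to the "Destructed" collision profile and plays a 2D fall sound (SC_Chute_Main) after a short delay.
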(event OnComponentBeginOverlap(Box)
  (params (OverlappedComponent :type Primitive%20Component%20Object%20Reference) (OtherActor :type Actor%20Object%20Reference) (OtherComp :type Primitive%20Component%20Object%20Reference) (OtherBodyIndex :type Integer) (bFromSweep :type Boolean) (SweepResult :type Hit%20Result%20Structure%20%28by%20ref%29))
  (bind _asbp_hero (Utilities|Casting|CastToBP_Hero OtherActor))
  (Class|DestructibleComponent|ApplyDamage (Variables|Default|GetDestructible) 1e+02 (Transformation|GetActorLocation self) (* (Transformation|GetActorUpVector _asbp_hero) -1.0) 0.0)
  (Collision|SetCollisionProfileName (Variables|Default|GetDestructible) "Destructed" true :!class /Script/Engine.PrimitiveComponent)
  (Utilities|FlowControl|Delay 1.8)
  (Audio|PlaySound2D "/Game/Sounds/Cue/Environnement/SC_Chute_Main.SC_Chute_Main" 1.0 1.0 0.0 0 0))

(event EventBeginPlay)

(event Collision|EventActorBeginOverlap
  (params (OtherActor :type Actor%20Object%20Reference)))

(event EventTick
  (params (DeltaSeconds :type Float%20%28single-precision%29)))

(fn ConstructionScript)