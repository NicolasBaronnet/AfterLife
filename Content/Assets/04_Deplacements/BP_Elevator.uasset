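; BP_Elevator is a lift that shuttles endlessly between BottomPoint and TopPoint once triggered by an actor overlap.
; The first overlap passes a DoOnce before the BP_Hero cast, then StartBot picks the initial direction.
; After WaitDuration, a looping timer at interval Speed teleports the lift in fixed Z steps without sweep.
; On reaching the target height, it clears that timer and starts the opposite direction.
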(event Custom|GoesUpTimer
  ;[1 1 1] Timer Go Top
  (if (> (.z (Transformation|GetActorLocation (Variables|Default|GetTopPoint))) (.z (Transformation|GetActorLocation self)))
    (Transformation|AddActorWorldOffset "0, 0,5.000000" false true)
    (else
      (Utilities|Time|ClearandInvalidateTimerbyHandle (Variables|Default|GetGoesUpTimerHandle))
      (CallFunction|GoesDown))))

(event Custom|GoesDown
  ;[1 1 1] Timer Go Down
  (Utilities|FlowControl|Delay (Variables|Default|GetWaitDuration))
  (bind _returnvalue (Utilities|Time|SetTimerbyEvent (delegate Custom|GoesDownTimer) (Variables|Default|GetSpeed) true))
  (Variables|Default|SetGoesDownTimerHandle _returnvalue))

(event Custom|GoesUp
  ;[1 1 1] Timer Go Top
  (Utilities|FlowControl|Delay (Variables|Default|GetWaitDuration))
  (bind _returnvalue (Utilities|Time|SetTimerbyEvent (delegate Custom|GoesUpTimer) (Variables|Default|GetSpeed) true))
  (Variables|Default|SetGoesUpTimerHandle _returnvalue))

(event Custom|GoesDownTimer
  ;[1 1 1] Timer Go Down
  (if (> (.z (Transformation|GetActorLocation self)) (.z (Transformation|GetActorLocation (Variables|Default|GetBottomPoint))))
    (Transformation|AddActorWorldOffset "0, 0,-5.000000" false true)
    (else
      (Utilities|Time|ClearandInvalidateTimerbyHandle (Variables|Default|GetGoesDownTimerHandle))
      (CallFunction|GoesUp))))

(event EventBeginPlay)

(event Collision|EventActorBeginOverlap
  (params (OtherActor :type Actor%20Object%20Reference))
  (Utilities|FlowControl|DoOnce false
    (:Completed
      (Utilities|Casting|CastToBP_Hero OtherActor)
      (if (Variables|Default|GetStartBot?)
        (CallFunction|GoesUp)
        (else
          (CallFunction|GoesDown))))))

(event EventTick
  (params (DeltaSeconds :type Float%20%28single-precision%29)))

(fn ConstructionScript)