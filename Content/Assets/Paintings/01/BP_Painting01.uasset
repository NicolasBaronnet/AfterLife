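; Painting prop Blueprint whose artwork is chosen per placed instance.
; The construction script reads the Material variable and assigns one of four painting materials to the first slot of its static mesh, with the fourth as the fallback for any other value.
; The event graph holds only disabled default events, so it has no runtime logic.
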(event EventBeginPlay)

(event Collision|EventActorBeginOverlap
  (params (OtherActor :type Actor%20Object%20Reference)))

(event EventTick
  (params (DeltaSeconds :type Float%20%28single-precision%29)))

(fn ConstructionScript
  (if (== (Variables|Default|GetMaterial) 1)
    (Rendering|Material|SetMaterial (Variables|Default|GetStaticMesh) 0 "/Game/Assets/Paintings/01/M_painting01.M_painting01")
    (elif (== (Variables|Default|GetMaterial) 2)
      (Rendering|Material|SetMaterial (Variables|Default|GetStaticMesh) 0 "/Game/Assets/Paintings/01/M_painting01_2.M_painting01_2")
      (elif (== (Variables|Default|GetMaterial) 3)
        (Rendering|Material|SetMaterial (Variables|Default|GetStaticMesh) 0 "/Game/Assets/Paintings/01/M_painting01_3.M_painting01_3")
        (else
          (Rendering|Material|SetMaterial (Variables|Default|GetStaticMesh) 0 "/Game/Assets/Paintings/01/M_painting01_4.M_painting01_4"))))))