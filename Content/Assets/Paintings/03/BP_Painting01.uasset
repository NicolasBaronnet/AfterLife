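; Painting prop Blueprint that displays one of four painting03 materials on its static mesh.
; The construction script checks the Material variable and assigns the matching material to slot 0, with the fourth serving as the fallback for any value other than 1 to 3.
; The event graph holds only disabled default events, so the painting has no runtime logic.
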(event EventBeginPlay)

(event Collision|EventActorBeginOverlap
  (params (OtherActor :type Actor%20Object%20Reference)))

(event EventTick
  (params (DeltaSeconds :type Float%20%28single-precision%29)))

(fn ConstructionScript
  (if (== (Variables|Default|GetMaterial) 1)
    (Rendering|Material|SetMaterial (Variables|Default|GetStaticMesh) 0 "/Game/Assets/Paintings/03/M_painting03_1.M_painting03_1")
    (elif (== (Variables|Default|GetMaterial) 2)
      (Rendering|Material|SetMaterial (Variables|Default|GetStaticMesh) 0 "/Game/Assets/Paintings/03/M_painting03_2.M_painting03_2")
      (elif (== (Variables|Default|GetMaterial) 3)
        (Rendering|Material|SetMaterial (Variables|Default|GetStaticMesh) 0 "/Game/Assets/Paintings/03/M_painting03_3.M_painting03_3")
        (else
          (Rendering|Material|SetMaterial (Variables|Default|GetStaticMesh) 0 "/Game/Assets/Paintings/03/M_painting03_4.M_painting03_4"))))))