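; End-game survival countdown that starts once when the Trigger is overlapped, then ends the level after its lights go out.
; Five chained timelines dim and narrow spotlight pairs in turn, while a looping timer plays spawn sounds at random lights.
; The last blackout kills enemies, resets the hero, and plays the cinematic with credits, then opens the menu when it finishes.
; Resetondeath stops the timelines, restores the lights and re-arms the trigger.
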(event Custom|OnActorBeginOverlap_Event_0
  (params (OverlappedActor :type Actor%20Object%20Reference) (OtherActor :type Actor%20Object%20Reference))
  (bind _lightsarray (Variables|Default|GetLightsArray))
  (bind _lightsarray_2 (Variables|Default|GetLightsArray))
  (bind _soundmanager (Variables|Default|GetSoundManager))
  (Utilities|FlowControl|DoOnce false
    (:Completed
      (Audio|PlaySoundatLocation "/Game/Sounds/Base/SD_Environnement/Spawn_enemie_loup/SC_SpawnLoup.SC_SpawnLoup" (Transformation|GetActorLocation (Utilities|Array|Get(acopy) _lightsarray_2 (Math|Random|RandomIntegerinRange 0 (- (Utilities|Array|Length _lightsarray_2) 1)))) "0, 0, 0" 1.0 1.0 0.0 0 0 0)
      (Utilities|FlowControl|Delay (Variables|Default|GetStartDelay))
      (Utilities|Casting|CastToBP_Hero OtherActor)
      (Utilities|FlowControl|Sequence
        (:then_0
          (|Closelight1)
          (|Closelight2)
          (|Closelight3)
          (|Closelight4)
          (|Closelight5)
          ;[1 1 1] End Level
          (bind _asbp_hero (Utilities|Casting|CastToBP_Hero (Game|Player|GetPlayerPawn 0)))
          (CameraFades|StartCameraFade :self (Game|GetPlayerCameraManager 0) :FromAlpha 1.0 :Duration 4.0 :bShouldFadeAudio true :bHoldWhenFinished true)
          (bind _asbp_hero_2 (Utilities|Casting|CastToBP_Hero (Game|Player|GetPlayerPawn 0)))
          (Default|EDResetRageHP _asbp_hero_2)
          (Variables|/Script/Engine.Actor|SetbCanBeDamaged _asbp_hero_2 false)
          (Default|StartGameSetUp _asbp_hero_2 false)
          (Variables|/Game/Enemies/BP_Spawner.BP_Spawner_C|SetSpawnNumber (Variables|Default|GetSpawnerRef) 0)
          (bind _outactors (Actor|GetAllActorsOfClass "/Game/Enemies/BP_Ennemi_Body.BP_Ennemi_Body_C"))
          (for _array_element _outactors
            (Default|DeathFunction _array_element))
          (bind _returnvalue (Sequencer|Player|CreateLevelSequencePlayer (Variables|Default|GetCinematic)))
          (Class|MovieSceneSequencePlayer|Playto _returnvalue)
          (bind _returnvalue_2 (UserInterface|CreateWidget "/Game/UI/UI_Credits.UI_Credits_C" (Game|GetPlayerController 0)))
          (UserInterface|Viewport|AddtoViewport _returnvalue_2 0)
          (Default|ChangeMusic _soundmanager "/Game/Sounds/Cue/Music/SC_Music_Ambiance_Banquet.SC_Music_Ambiance_Banquet")
          (Default|NewAmbiance _soundmanager))
        (:then_1
          ;[1 1 1] Play Sound every 20 sec
          (bind _returnvalue_3 (Utilities|Time|SetTimerbyEvent (delegate Custom|Play%20sound%20event) 2e+01 true))
          (Variables|Default|SetPlaySoundEventTimerHandle _returnvalue_3)
          (Audio|PlaySoundatLocation "/Game/Sounds/Base/SD_Environnement/Spawn_enemie_loup/SC_SpawnLoup.SC_SpawnLoup" (Transformation|GetActorLocation (Utilities|Array|Get(acopy) _lightsarray (Math|Random|RandomIntegerinRange 0 (- (Utilities|Array|Length _lightsarray) 1)))) "0, 0, 0" 1.0 1.0 0.0 0 0 0))))))

(event Custom|Reset%20on%20death
  (bind _lightsarray (Variables|Default|GetLightsArray))
  (bind _lightsarray_2 (Variables|Default|GetLightsArray))
  (bind _soundmanager (Variables|Default|GetSoundManager))
  (Utilities|FlowControl|Sequence
    (:then_0
      (|Closelight1) ; enters at Stop
    )
    (:then_1
      (|Closelight2) ; enters at Stop
    )
    (:then_2
      (|Closelight3) ; enters at Stop
    )
    (:then_3
      (|Closelight4) ; enters at Stop
    )
    (:then_4
      (|Closelight5) ; enters at Stop
    )
    (:then_6
      (Utilities|FlowControl|Delay 1.0)
      (for _array_element (Variables|Default|GetLightsArray)
        (Default|SetIntensity _array_element (Variables|Default|GetInitialIntensity))
        (Default|ResetConesAnlges _array_element))
      (Utilities|Time|ClearandInvalidateTimerbyHandle (Variables|Default|GetPlaySoundEventTimerHandle))
      (Utilities|FlowControl|DoOnce false) ; enters at Reset
    )))

(event Custom|Play%20sound%20event
  (bind _lightsarray (Variables|Default|GetLightsArray))
  ;[1 1 1] Play Sound every 20 sec
  (Audio|PlaySoundatLocation "/Game/Sounds/Base/SD_Environnement/Spawn_enemie_loup/SC_SpawnLoup.SC_SpawnLoup" (Transformation|GetActorLocation (Utilities|Array|Get(acopy) _lightsarray (Math|Random|RandomIntegerinRange 0 (- (Utilities|Array|Length _lightsarray) 1)))) "0, 0, 0" 1.0 1.0 0.0 0 0 0))

(event Custom|CustomEvent_0
  (Game|OpenLevel(byName) "Ana_Test_Menu"))

(event EventBeginPlay
  (EventDispatchers|AssignOnActorBeginOverlap (Variables|Default|GetTrigger) (delegate Custom|OnActorBeginOverlap_Event_0))
  (EventDispatchers|BindEventtoOnFinished (stale Custom|OnActorBeginOverlap_Event_0 _returnvalue) (delegate Custom|CustomEvent_0)))

(event EventTick
  (params (DeltaSeconds :type Float%20%28single-precision%29)))

(fn ConstructionScript)