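; Player hero character with cursor-driven top-down combat: toggles between travel and armed modes, re-socketing axe and shield.
; A CharacBehavior state struct gates keyboard movement, cursor aiming, a timer-charged impulse dash, a spinning axe hit and parry.
; Tick handles rotation, the debug aim arrow and speed-based dash recovery, while overlap boxes deal damage.
; Game mode dispatchers broadcast action, rage and death events and trigger a brief stun on damage.
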(event OnComponentBeginOverlap(DashDamagesBox)
  (params (OverlappedComponent :type Primitive%20Component%20Object%20Reference) (OtherActor :type Actor%20Object%20Reference) (OtherComp :type Primitive%20Component%20Object%20Reference) (OtherBodyIndex :type Integer) (bFromSweep :type Boolean) (SweepResult :type Hit%20Result%20Structure%20%28by%20ref%29))
  (bind _chargedamages (Variables|Dash|GetChargeDamages))
  ;[1 1 1] Dash Dammages
  (if (.InDash (Utilities|Struct|BreakS_States (Variables|CharacterAttributes|GetCharacBehavior)))
    (Game|Damage|ApplyDamage OtherActor _chargedamages 0 0 "/Script/Engine.DamageType")
    (Game|Damage|ApplyRadialDamage _chargedamages (Math|Vector|GetForwardVector (Variables|Character|GetMesh)) 5e+01 "/Script/Engine.DamageType" 0 0 0 true "ECC_Visibility")))

(event OnComponentBeginOverlap(AxeDamagesBox)
  (params (OverlappedComponent :type Primitive%20Component%20Object%20Reference) (OtherActor :type Actor%20Object%20Reference) (OtherComp :type Primitive%20Component%20Object%20Reference) (OtherBodyIndex :type Integer) (bFromSweep :type Boolean) (SweepResult :type Hit%20Result%20Structure%20%28by%20ref%29))
  (bind _chargedamages (Variables|Dash|GetChargeDamages))
  ;[1 1 1] Axe Damages
  (if (.InAxeHit (Utilities|Struct|BreakS_States (Variables|CharacterAttributes|GetCharacBehavior)))
    (Game|Damage|ApplyDamage OtherActor _chargedamages 0 0 "/Script/Engine.DamageType")
    (Game|Damage|ApplyRadialDamage _chargedamages (Math|Vector|GetForwardVector (Variables|Character|GetMesh)) 5e+01 "/Script/Engine.DamageType" 0 0 0 true "ECC_Visibility")))

(event Custom|EDTakeDamages_Event_0
  ;[1 1 1] BEGIN PLAY
  (if (.CanTakeDAmages (Utilities|Struct|BreakS_States (Variables|CharacterAttributes|GetCharacBehavior)))
    (Variables|CharacterAttributes|SetCharacBehavior (Utilities|Struct|MakeS_States false false false false false true))
    (Utilities|FlowControl|Delay 0.5)
    (Variables|CharacterAttributes|SetCharacBehavior (Utilities|Struct|MakeS_States true true true true true true))))

(event Custom|ArmedState
  ;[1 1 1] BEGIN PLAY
  ;;[1 1 1] Bind Armed
  (Utilities|FlowControl|FlipFlop
    (:A
      (Variables|CharacterAttributes|SetCharacBehavior (Utilities|Struct|MakeS_States true true true true true true)))
    (:B
      (Variables|CharacterAttributes|SetCharacBehavior (Utilities|Struct|MakeS_States true false true)))))

(event Custom|ChargeDash
  ;[1 1 1] CONTROLS
  ;;[1 1 1] Dash
  (Math|Integer|IncrementInt (Variables|Dash|GetDashRange)))

(event EventBeginPlay
  ;[1 1 1] BEGIN PLAY
  (Variables|Default|SetGameMod (CallFunction|GetGameMod))
  (Variables|/Script/Engine.PlayerController|SetbShowMouseCursor (Game|GetPlayerController 0) true)
  (Utilities|FlowControl|Sequence
    (:then_0
      ;;[1 1 1] Bind Armed
      (EventDispatchers|BindEventtoEDIsArmed (Variables|Default|GetGameMod) (delegate Custom|ArmedState)))
    (:then_1
      ;;[1 1 1] Create UI
      (bind _returnvalue (UserInterface|CreateWidget "/Game/UI/UI_Main.UI_Main_C"))
      (UserInterface|Viewport|AddtoViewport _returnvalue 0))
    (:then_2
      (EventDispatchers|AssignEDTakeDamages (Variables|Default|GetGameMod) (delegate Custom|EDTakeDamages_Event_0)))))

(event EventTick
  (params (DeltaSeconds :type Float%20%28single-precision%29))
  (bind _returnvalue (Game|GetPlayerController 0))
  (bind _returnvalue_2 (Transformation|GetActorRotation))
  (bind _hitresult (Game|Player|GetHitResultUnderCursorbyChannel _returnvalue "TraceTypeQuery1" true))
  (bind (_bblockinghit _binitialoverlap _time _distance _location _impactpoint _normal) (Collision|BreakHitResult _hitresult))
  ;[1 1 1] TICK
  (Variables|Default|SetWorldTick DeltaSeconds)
  (Utilities|FlowControl|Sequence
    (:then_0
      ;;[1 1 1] Orient Player With mouse
      (if (and (.CanWalk (Utilities|Struct|BreakS_States (Variables|CharacterAttributes|GetCharacBehavior))) (.IsArmed (Utilities|Struct|BreakS_States (Variables|CharacterAttributes|GetCharacBehavior))))
        (Variables|Controller|SetmousePos _location)
        (if (Math|Vector|Equal(Vector) _normal "0, 0,1.000000" 0.1)
          (Transformation|SetActorRotation (Math|Rotator|MakeRotator (.roll _returnvalue_2) (.pitch _returnvalue_2) (.yaw (Math|Rotator|FindLookatRotation (Transformation|GetActorLocation) _location)))))))
    (:then_1
      (CallFunction|GetSpeed)
      ;;[1 1 1] Character Orientation with Keyboard
      (if (and (.CanWalk (Utilities|Struct|BreakS_States (Variables|CharacterAttributes|GetCharacBehavior))) (not (.IsArmed (Utilities|Struct|BreakS_States (Variables|CharacterAttributes|GetCharacBehavior)))))
        (bind _output_get (Variables|Controller|SetForwardRef (Math|Vector|MakeVector (Variables|Controller|GetMoveRight) (Variables|Controller|GetMoveForward) 0.0)))
        (bind _returnvalue_3 (CallFunction|GetDirectionAngle _output_get))
        (if (Math|Float|InRange(Float) _returnvalue_3 0.0 1.8e+02)
          (if (not (Math|Float|NearlyEqual(Float) _returnvalue_3 0.0 1e+01))
            (Transformation|AddActorLocalRotation "0,7.000000, 0" false false))
          (elif (not (Math|Float|NearlyEqual(Float) _returnvalue_3 0.0 1e+01))
            (Transformation|AddActorLocalRotation "0,-7.000000, 0" false false)))))
    (:then_2
      (Utilities|FlowControl|Sequence
        (:then_0
          ;;[1 1 1] Aiming Arrow
          (if (and (Variables|Dash|GetDrawArrow) (.IsArmed (Utilities|Struct|BreakS_States (Variables|CharacterAttributes|GetCharacBehavior))))
            (Rendering|Debug|DrawDebugArrow :LineStart (Transformation|GetActorLocation self) :LineEnd (Variables|Controller|GetmousePos) :ArrowSize 1e+01 :Duration (* (Variables|Default|GetWorldTick) 3.0) :Thickness 5.0)))
        (:then_1
          ;;[1 1 1] End dash conditions, recover character Control
          (if (Math|Boolean|ANDBoolean (< (Variables|CharacterAttributes|GetPlayerSpeed) 1.5e+02) (.IsArmed (Utilities|Struct|BreakS_States (Variables|CharacterAttributes|GetCharacBehavior))) (.InDash (Utilities|Struct|BreakS_States (Variables|CharacterAttributes|GetCharacBehavior))))
            (Utilities|FlowControl|DoOnce false :!label _label
              (:Completed
                (Default|CallEDEndDash (Variables|Default|GetGameMod))
                (Utilities|FlowControl|Delay (Variables|Dash|GetRecoverTime))
                (Variables|CharacterAttributes|SetCharacBehavior (Utilities|Struct|MakeS_States true true true true false true))
                (Default|CallEDWalking (CallFunction|GetGameMod))
                (Input|EnableInput (Game|GetPlayerController 0))
                (Collision|SetCollisionResponsetoChannel (Variables|Collision|GetCapsuleComponent) "ECC_Destructible" "ECR_Block")
                (Variables|/Script/Engine.CharacterMovementComponent|SetMaxWalkSpeed (Variables|Character|GetCharacterMovement) (Variables|Movements|GetFightRunSpeed))
                (Default|CallEDEndDash (Variables|Default|GetGameMod))
                (goto _label Reset)))))))
    (:then_3
      ;;[1 1 1] Mouvement durant l'animation de dash
      (if (.InAxeHit (Utilities|Struct|BreakS_States (Variables|CharacterAttributes|GetCharacBehavior)))
        (Pawn|Input|AddMovementInput (Math|Vector|Normalize (Math|Vector|GetUnitDirection(Vector) (Transformation|GetWorldLocation (Variables|Character|GetMesh)) (Variables|Controller|GetmousePos))) (Variables|AnimationFlow|GetMovementDuringHit) false)
        (Transformation|AddLocalRotation (Variables|Character|GetMesh) (Math|Rotator|MakeRotator 0.0 0.0 (/ 3.6e+02 (/ (Variables|AnimationFlow|GetSwordHitTime) (Variables|Default|GetWorldTick)))) false false)))))

(event Input|ActionEvents|InputActionDash
  (params (Key :type Key%20Structure :default "None"))
  ;[1 1 1] CONTROLS
  ;;[1 1 1] Dash
  (:Pressed
    (if (.IsArmed (Utilities|Struct|BreakS_States (Variables|CharacterAttributes|GetCharacBehavior)))
      (Variables|Dash|SetDrawArrow true)
      (Variables|CharacterAttributes|SetCharacBehavior (Utilities|Struct|MakeS_States true true false true false true))
      (Variables|/Script/Engine.CharacterMovementComponent|SetMaxWalkSpeed (Variables|Character|GetCharacterMovement) (Variables|Movements|GetDashPreparationSpeed))
      (bind _returnvalue (Utilities|Time|SetTimerbyEvent (delegate Custom|ChargeDash) 0.05 true))
      (Variables|Dash|SetDashTimer _returnvalue)))
  (:Released
    (if (.IsArmed (Utilities|Struct|BreakS_States (Variables|CharacterAttributes|GetCharacBehavior)))
      (Variables|Dash|SetDrawArrow false)
      (Variables|CharacterAttributes|SetCharacBehavior (Utilities|Struct|MakeS_States false false false false false true true))
      (Input|DisableInput (Game|GetPlayerController 0))
      (if (Utilities|Time|IsValidTimerHandle (Variables|Dash|GetDashTimer))
        (Utilities|Time|ClearandInvalidateTimerbyHandle (Variables|Dash|GetDashTimer))
        (Physics|AddImpulse (Variables|Character|GetCharacterMovement) (* (Math|Vector|GetUnitDirection(Vector) (Transformation|GetActorLocation self) (Variables|Controller|GetmousePos)) (* (Variables|Dash|GetDashSpeed) (Variables|Dash|GetDashRange))) true)
        (Variables|Dash|SetDashRange 0)
        (Collision|SetCollisionResponsetoChannel (Variables|Collision|GetCapsuleComponent) "ECC_Destructible" "ECR_Overlap")
        (Default|CallEDIsCharging? (CallFunction|GetGameMod))
        (Default|CallEDRageDash (Variables|Default|GetGameMod))))))

(event Input|ActionEvents|InputActionArmed
  (params (Key :type Key%20Structure :default "None"))
  ;[1 1 1] CONTROLS
  ;;[1 1 1] Is Armed Variable
  (:Pressed
    (Utilities|FlowControl|FlipFlop
      (:A
        (Variables|/Script/Engine.CharacterMovementComponent|SetMaxWalkSpeed (Variables|Character|GetCharacterMovement) (Variables|Movements|GetFightRunSpeed))
        (Variables|CharacterAttributes|SetCharacBehavior (Utilities|Struct|MakeS_States true true true true true true))
        (Transformation|AttachComponentToComponent (Variables|Default|GetSM_Axe) (Variables|Character|GetMesh) "WeaponSocket" "SnapToTarget" "SnapToTarget" "KeepWorld" true)
        (Transformation|AttachComponentToComponent (Variables|Default|GetSM_Shield) (Variables|Character|GetMesh) "ShieldSocket" "SnapToTarget" "SnapToTarget" "KeepWorld" true)
        (Default|CallEDIsArmed (Variables|Default|GetGameMod)))
      (:B
        (Variables|/Script/Engine.CharacterMovementComponent|SetMaxWalkSpeed (Variables|Character|GetCharacterMovement) (Variables|Movements|GetTravellingRunSpeed))
        (Variables|CharacterAttributes|SetCharacBehavior (Utilities|Struct|MakeS_States true false false true))
        (Transformation|AttachComponentToComponent (Variables|Default|GetSM_Axe) (Variables|Character|GetMesh) "TidyWeaponSocket" "SnapToTarget" "SnapToTarget" "KeepWorld" true)
        (Transformation|AttachComponentToComponent (Variables|Default|GetSM_Shield) (Variables|Character|GetMesh) "TidyShieldSocket" "SnapToTarget" "SnapToTarget" "KeepWorld" true)
        (Default|CallEDIsArmed (Variables|Default|GetGameMod))))))

(event Input|ActionEvents|InputActionWalk
  (params (Key :type Key%20Structure :default "None"))
  ;[1 1 1] CONTROLS
  ;;[1 1 1] Walk
  (:Pressed
    (Variables|/Script/Engine.CharacterMovementComponent|SetMaxWalkSpeed (Variables|Character|GetCharacterMovement) (Variables|Movements|GetDefaultWalkSpeed)))
  (:Released
    (Variables|/Script/Engine.CharacterMovementComponent|SetMaxWalkSpeed (Variables|Character|GetCharacterMovement) (Variables|Movements|GetFightRunSpeed))))

(event Input|ActionEvents|InputActionAxeHit
  (params (Key :type Key%20Structure :default "None"))
  (bind _characbehavior (Variables|CharacterAttributes|GetCharacBehavior))
  (bind (_canwalk _candash _canparry _cantakedamages _canhit _isarmed) (Utilities|Struct|BreakS_States _characbehavior))
  ;[1 1 1] CONTROLS
  ;;[1 1 1] Input AxeHit
  (:Pressed
    (if (and _canwalk _isarmed)
      (CallFunction|AxeHitFunction)
      (Utilities|FlowControl|Delay (Variables|AnimationFlow|GetSwordHitTime))
      (CallFunction|AxeHitFunction)
      (Transformation|SetRelativeRotation (Variables|Character|GetMesh) "0,-90.000000, 0" false false)
      (Default|CallEDWalking (Variables|Default|GetGameMod))
      (Default|CallEDRageAxe (Variables|Default|GetGameMod)))))

(event Input|ActionEvents|InputActionParry
  (params (Key :type Key%20Structure :default "None"))
  ;[1 1 1] CONTROLS
  ;;[1 1 1] KeyBinding Parry
  (:Pressed
    (if (.CanParry (Utilities|Struct|BreakS_States (Variables|CharacterAttributes|GetCharacBehavior)))
      (CallFunction|ParryFunction)
      (Default|CallEDRageShield (Variables|Default|GetGameMod))))
  (:Released
    (if (.InParry (Utilities|Struct|BreakS_States (Variables|CharacterAttributes|GetCharacBehavior)))
      (CallFunction|ParryFunction))))

(event Input|AxisEvents|InputAxisMoveForward
  (params (AxisValue :type Float%20%28single-precision%29))
  ;[1 1 1] CONTROLS
  ;;[1 1 1] Movements Controls
  (bind _output_get (Variables|Controller|SetMoveForward AxisValue))
  (if (.CanWalk (Utilities|Struct|BreakS_States (Variables|CharacterAttributes|GetCharacBehavior)))
    (Pawn|Input|AddMovementInput "0.000000,1.000000, 0" _output_get false)))

(event Input|AxisEvents|InputAxisMoveRight
  (params (AxisValue :type Float%20%28single-precision%29))
  ;[1 1 1] CONTROLS
  ;;[1 1 1] Movements Controls
  (bind _output_get (Variables|Controller|SetMoveRight AxisValue))
  (if (.CanWalk (Utilities|Struct|BreakS_States (Variables|CharacterAttributes|GetCharacBehavior)))
    (Pawn|Input|AddMovementInput "1.000000,0.000000, 0" _output_get false)))

(fn ConstructionScript
  (Transformation|AttachComponentToComponent (Variables|Default|GetSM_Axe) (Variables|Character|GetMesh) "TidyWeaponSocket" "SnapToTarget" "SnapToTarget" "KeepWorld" true)
  (Transformation|AttachComponentToComponent (Variables|Default|GetSM_Shield) (Variables|Character|GetMesh) "TidyShieldSocket" "SnapToTarget" "SnapToTarget" "KeepWorld" true)
  (Variables|CharacterAttributes|SetCharacBehavior (Utilities|Struct|MakeS_States true true true true true)))

(fn GetSpeed
  (bind _self self)
  (bind _returnvalue (Transformation|GetVelocity _self))
  (Variables|CharacterAttributes|SetPlayerSpeed (Math|Float|Sqrt (+ (Math|Float|Square (.x _returnvalue)) (Math|Float|Square (.y _returnvalue))))))

(fn CompareSpeed
  (params (Speed :type Float%20%28single-precision%29))
  (if (and (< (LocalVariables|GetpreviousSpeed) Speed) (Math|Float|InRange(Float) Speed 7.5e+02 6.5e+02))
    (bind _output_get (LocalVariables|Setdisable false))
    (LocalVariables|SetpreviousSpeed Speed)
    (else
      (LocalVariables|Setdisable true)
      (LocalVariables|SetpreviousSpeed Speed)))
  (return _output_get))

(fn GetDirectionAngle
  (params (A :type Vector))
  (bind _returnvalue (Transformation|GetActorForwardVector))
  (bind _returnvalue_2 (Math|Vector|Normalize A))
  (bind _returnvalue_3 (Math|Vector|Normalize _returnvalue))
  (return (* (Class|KismetMathLibrary|DegAcos (Math|Vector|DotProduct _returnvalue_3 _returnvalue_2)) (Math|Float|Sign(Float) (.z (Math|Vector|CrossProduct _returnvalue_3 _returnvalue_2))))))

(fn Death
  (Utilities|FlowControl|Sequence
    (:then_0
      (Default|CallEDDeath (Variables|Default|GetGameMod)))
    (:then_1
      (Input|DisableInput (Game|GetPlayerController 0)))))

(fn AxeHitFunction
  (if (not (.InAxeHit (Utilities|Struct|BreakS_States (Variables|CharacterAttributes|GetCharacBehavior))))
    (Input|DisableInput (Game|GetPlayerController 0))
    (Variables|CharacterAttributes|SetCharacBehavior (Utilities|Struct|MakeS_States false false false true false true false false true))
    (Default|CallEDAxeHit (CallFunction|GetGameMod))
    (else
      (Input|EnableInput (Game|GetPlayerController 0))
      (Variables|CharacterAttributes|SetCharacBehavior (Utilities|Struct|MakeS_States true true true true true true))
      (Default|CallEDAxeHit (CallFunction|GetGameMod))))
  (Variables|AxeHit|SetAxeHitDirection (Variables|Controller|GetmousePos))
  (return))

(fn ParryFunction
  (if (.InParry (Utilities|Struct|BreakS_States (Variables|CharacterAttributes|GetCharacBehavior)))
    (Variables|CharacterAttributes|SetCharacBehavior (Utilities|Struct|MakeS_States true true true true true true))
    (else
      (Variables|CharacterAttributes|SetCharacBehavior (Utilities|Struct|MakeS_States false false false false true true false true)))))

(fn LifeGestureFunction
  (params (Count :type Integer))
  (Variables|CharacterAttributes|SetHP (+ Count (Variables|CharacterAttributes|GetHP)))
  (if (<= (Variables|CharacterAttributes|GetHP) 0)
    (CallFunction|Death)))