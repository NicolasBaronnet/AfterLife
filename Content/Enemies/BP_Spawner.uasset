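; Room encounter spawner that locks the hero in with Errinye and Starven enemies.
; Entering the trigger lowers doors, briefly freezes the hero, clears leftover enemy bodies and spawns the initial enemies at random points.
; Each enemy death event spawns one replacement while stock remains, using SortArray to favor the point farthest from the player.
; Once the remaining-enemy counter runs out, doors rise, dash is disabled and any linked elevator is enabled.
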(event Custom|EDEnnemiDeath_Event_0
  (bind _elevator (Variables|Default|GetElevator))
  ;[1 1 1] Chose far away spawn point
  (if (Variables|Default|GetEnabled)
    (Utilities|FlowControl|Sequence
      (:then_0
        (if (> (Variables|Default|GetSpawnNumber) 0)
          (CallFunction|SortArray)
          (Variables|Default|SetSimultaneaousSpawn (Math|Random|RandomIntegerinRange 1 2))
          (for _index (range 0 0)
            (if (and (== (Math|Random|RandomIntegerinRange 0 (Variables|Default|GetErrinyeSpawnRate)) 0) (Variables|Default|GetHasErrinye?))
              (AI|SpawnAIFromClass "/Game/Enemies/02_Errinye/BP_Errinye.BP_Errinye_C" "/Game/Enemies/02_Errinye/BT_Errinye.BT_Errinye" (Transformation|GetActorLocation (Utilities|Array|Get(acopy) (Variables|Default|GetSpawnerLoc) _index)) "0, 0, 0" false 0)
              (else
                (AI|SpawnAIFromClass "/Game/Enemies/01_Starved/BP_Starven.BP_Starven_C" "/Game/Enemies/01_Starved/BT_Starven.BT_Starven" (Transformation|GetActorLocation (Utilities|Array|Get(acopy) (Variables|Default|GetSpawnerLoc) _index)) "0, 0, 0" false 0)))
            (Math|Integer|DecrementInt (Variables|Default|GetSpawnNumber)))))
      (:then_1
        (Math|Integer|DecrementInt (Variables|Default|GetRemainsEnnemies)
          (:%20%20
            (if (< (Variables|Default|GetRemainsEnnemies) -1)
              (Utilities|FlowControl|Delay 2.0)
              (bind _asbp_hero (Utilities|Casting|CastToBP_Hero (Game|Player|GetPlayerPawn 0)))
              (Variables|/Game/Hero/BP_Hero.BP_Hero_C|SetCharacBehavior _asbp_hero (Utilities|Struct|MakeS_States true false))
              (for _array_element (Variables|Default|GetDoors)
                (Default|GoesUp _array_element))
              (Utilities|IsValid _elevator
                (:Is%20Valid
                  (Variables|/Game/Assets/04_Deplacements/BP_Elevator.BP_Elevator_C|SetEnabled? _elevator true))))))))))

(event Custom|OnActorBeginOverlap_Event_0
  (params (OverlappedActor :type Actor%20Object%20Reference) (OtherActor :type Actor%20Object%20Reference))
  ;[1 1 1] Close doors
  (Utilities|FlowControl|DoOnce false
    (:Completed
      (Variables|Default|SetEnabled true)
      (bind _asbp_hero (Utilities|Casting|CastToBP_Hero OtherActor))
      (Utilities|FlowControl|Sequence
        (:then_0
          (Variables|/Game/Hero/BP_Hero.BP_Hero_C|SetCharacBehavior _asbp_hero (Utilities|Struct|MakeS_States false false))
          (for _array_element (Variables|Default|GetDoors)
            (Default|GoesDown _array_element))
          ;[1 1 1] Spawn Initial
          (Utilities|FlowControl|Delay (Variables|Default|GetDuration))
          (Variables|/Game/Hero/BP_Hero.BP_Hero_C|SetCharacBehavior _asbp_hero (Utilities|Struct|MakeS_States true true true true true true))
          (Utilities|FlowControl|Delay (Variables|Default|GetInitialSpawnDelay))
          (for _index (range 0 (Variables|Default|GetInitialErrinyes))
            (Game|SpawnActorfromClass "/Game/Enemies/02_Errinye/BP_Errinye.BP_Errinye_C" (Transformation|GetActorTransform (Utilities|Array|Get(acopy) (Variables|Default|GetSpawnerLoc) (Math|Random|RandomIntegerinRange 0 (- (Utilities|Array|Length (Variables|Default|GetSpawnerLoc)) 1)))) "Undefined" 0 "/Game/Plugs_In/Props/Materials/M_Shelf.M_Shelf" "/Game/Plugs_In/Props/Materials/M_Shelf.M_Shelf" 0))
          (for _index_2 (range 0 (Variables|Default|GetInitialStarven))
            (Game|SpawnActorfromClass "/Game/Enemies/01_Starved/BP_Starven.BP_Starven_C" (Transformation|GetActorTransform (Utilities|Array|Get(acopy) (Variables|Default|GetSpawnerLoc) (Math|Random|RandomIntegerinRange 0 (- (Utilities|Array|Length (Variables|Default|GetSpawnerLoc)) 1)))) "Undefined" 0 "/Game/Materials/Blocking_MAterials/M_Red.M_Red" "/Game/Plugs_In/Props/Materials/M_Shelf.M_Shelf" 0)))
        (:then_1
          ;;[1 1 1] Détruire les corps inutilisés
          (bind _outactors (Actor|GetAllActorsOfClass "/Game/Enemies/BP_Ennemi_Body.BP_Ennemi_Body_C"))
          (for _array_element_2 _outactors
            (Actor|DestroyActor _array_element_2)))))))

(event EventBeginPlay
  (bind _triggerdentreesalle (Variables|Default|GetTriggerDentreeSalle))
  (Utilities|FlowControl|Sequence
    (:then_0
      ;[1 1 1] Chose far away spawn point
      (EventDispatchers|AssignEDEnnemiDeath (CallFunction|GetGameMod) (delegate Custom|EDEnnemiDeath_Event_0))
      (Variables|Default|SetRemainsEnnemies (+ (Variables|Default|GetSpawnNumber) (Variables|Default|GetInitialStarven) (Variables|Default|GetInitialErrinyes))))
    (:then_1
      ;[1 1 1] Close doors
      (Utilities|IsValid _triggerdentreesalle
        (:Is%20Valid
          (EventDispatchers|AssignOnActorBeginOverlap _triggerdentreesalle (delegate Custom|OnActorBeginOverlap_Event_0)))))))

(event Collision|EventActorBeginOverlap
  (params (OtherActor :type Actor%20Object%20Reference)))

(fn ConstructionScript)

(fn SortArray
  (bind _distancespawner (Variables|Default|GetDistanceSpawner))
  (bind _distancespawner_2 (Variables|Default|GetDistanceSpawner))
  (for _array_element (Variables|Default|GetSpawnerLoc)
    (Utilities|Array|Add _distancespawner (Transformation|GetDistanceTo _array_element (Game|Player|GetPlayerPawn 0))))
  (for (_array_element_2 _array_index) _distancespawner
    (for _index (range _array_index (- (Utilities|Array|Length (Variables|Default|GetDistanceSpawner)) 1))
      (if (> (Utilities|Array|Get(acopy) _distancespawner_2 _index) _array_element_2)
        (Utilities|Array|Swap _distancespawner_2 _index _array_index)
        (Utilities|Array|Swap (Variables|Default|GetSpawnerLoc) _index _array_index)))))