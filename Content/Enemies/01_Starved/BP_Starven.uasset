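; BP_Starven is the Blueprint for the Starved enemy, providing its eye-light flash and death audio.
; The EyesLighting event shows two spotlights, then hides them after a short delay.
; The DeathSound event plays the starve death sound at the actor's location.
; Neither event is called within these graphs, and the default BeginPlay, overlap and Tick events are disabled.
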(event EventBeginPlay
  (|CallParentFunction) ; This node is disabled and will not be called.\nDrag off pins to build functionality.
)

(event Collision|EventActorBeginOverlap
  (params (OtherActor :type Actor%20Object%20Reference))
  (|CallParentFunction OtherActor) ; This node is disabled and will not be called.\nDrag off pins to build functionality.
)

(event EventTick
  (params (DeltaSeconds :type Float%20%28single-precision%29))
  (|CallParentFunction DeltaSeconds) ; This node is disabled and will not be called.\nDrag off pins to build functionality.
)

(event EventEyesLighting
  (Rendering|SetVisibility (Variables|Default|GetSpotLight1) true false)
  (Utilities|FlowControl|Delay 0.7)
  (Rendering|SetVisibility (Variables|Default|GetSpotLight1) false false))

(event EventDeathSound
  (Audio|PlaySoundatLocation "/Game/Sounds/Cue/Gameplay/Starven/SC_StarveDeath.SC_StarveDeath" (Transformation|GetActorLocation) "0, 0, 0" 1.0 1.0 0.0 0 0 0))

(fn ConstructionScript
  (|CallParentFunction))