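; Enemy Blueprint that hands its behavior to an AI controller running the BT_Enemy behavior tree.
; On BeginPlay it starts the tree, then writes the player character's mesh location to the PlayerLocation blackboard key once, with no later refresh.
; It also sets the SelfObject blackboard key, with no object value shown.
; Tick, overlap and construction logic are empty.
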(event EventBeginPlay
  (bind _self self)
  (bind _returnvalue (AI|GetBlackboard _self))
  (AI|RunBehaviorTree (AI|GetAIController _self) "/Game/Enemies/BT_Enemy.BT_Enemy")
  (bind _output_get (Variables|Default|SetBlackBoardRef _returnvalue))
  (AI|Components|Blackboard|SetValueasVector _output_get (Utilities|Name|MakeLiteralName "PlayerLocation") (Transformation|GetWorldLocation (Variables|/Script/Engine.Character|GetMesh (Game|GetPlayerCharacter 0))))
  (AI|Components|Blackboard|SetValueasObject _returnvalue (Variables|Default|GetSelfObject) 0))

(event Collision|EventActorBeginOverlap
  (params (OtherActor :type Actor%20Object%20Reference)))

(event EventTick
  (params (DeltaSeconds :type Float%20%28single-precision%29)))

(fn ConstructionScript)