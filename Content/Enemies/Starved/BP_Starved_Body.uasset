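; BP_Starved_Body is the body Blueprint of the Starved enemy and tracks whether the hero is within attack range.
; It caches the player's BP_Hero on BeginPlay, while a Box component's overlap events store the hero's capsule as ObjectInAttackRange.
; The reference clears when that capsule leaves the box, or when any non-hero actor begins overlapping it.
; No attack logic runs here.
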(event OnComponentBeginOverlap(Box)
  (params (OverlappedComponent :type Primitive%20Component%20Object%20Reference) (OtherActor :type Actor%20Object%20Reference) (OtherComp :type Primitive%20Component%20Object%20Reference) (OtherBodyIndex :type Integer) (bFromSweep :type Boolean) (SweepResult :type Hit%20Result%20Structure%20%28by%20ref%29))
  ;[1 1 1] Ovelapped capsule in attack range Gesture
  (bind _asbp_hero (Utilities|Casting|CastToBP_Hero OtherActor)
    (:then
      (if (== (Variables|/Script/Engine.Character|GetCapsuleComponent _asbp_hero) OtherComp)
        (Variables|Default|SetObjectInAttackRange OtherComp)))
    (:CastFailed
      (Variables|Default|SetObjectInAttackRange 0))))

(event OnComponentEndOverlap(Box)
  (params (OverlappedComponent :type Primitive%20Component%20Object%20Reference) (OtherActor :type Actor%20Object%20Reference) (OtherComp :type Primitive%20Component%20Object%20Reference) (OtherBodyIndex :type Integer))
  ;[1 1 1] Ovelapped capsule in attack range Gesture
  (if (== OtherComp (Variables|Default|GetObjectInAttackRange))
    (Variables|Default|SetObjectInAttackRange 0)))

(event EventBeginPlay
  ;[1 1 1] Get ref player
  (bind _asbp_hero (Utilities|Casting|CastToBP_Hero (Game|Player|GetPlayerPawn 0)))
  (Variables|Default|SetPlayerRef _asbp_hero))

(event Collision|EventActorBeginOverlap
  (params (OtherActor :type Actor%20Object%20Reference)))

(event EventTick
  (params (DeltaSeconds :type Float%20%28single-precision%29)))

(fn ConstructionScript)