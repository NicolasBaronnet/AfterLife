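; BP_MonsterAnger is an enemy that patrols at a slower speed until PawnSensing first sees a pawn, then enters combat at max speed with a detection sound.
; Tick tracks speed and distance to the player, triggering a jump attack when in range, in combat and available.
; Separate timelines drive the jump, moving the actor with sweep and offsetting the mesh.
; Nothing here re-enables the jump afterward.
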(event Custom|OnSeePawn_Event_0
  (params (Pawn :type Pawn%20Object%20Reference))
  ;[1 1 1] Bind Event On see
  (Utilities|FlowControl|DoOnce false
    (:Completed
      (Variables|Default|SetInFight? true)
      (Audio|PlaySound2D "/Game/Sounds/DetectedSound.DetectedSound" 1.0 1.0 0.0 0 0)
      (Variables|/Script/Engine.CharacterMovementComponent|SetMaxWalkSpeed (Variables|Character|GetCharacterMovement) (Variables|Default|GetMaxSpeed)))))

(event Custom|JumpAttack
  (bind _mesh (Variables|Character|GetMesh))
  (Utilities|FlowControl|Sequence
    (:then_0
      (Utilities|FlowControl|Delay 0.4)
      (bind _jumpdirection (Timeline|JumpEvent PlayFromStart)
        (:Update
          (Transformation|AddActorLocalOffset _jumpdirection true false))
        (:Finished
          (Variables|Default|SetJumpAvailable false)
          (Variables|Default|SetJumpAttackStart false)
          (Utilities|FlowControl|DoOnce false) ; enters at Reset
        )))
    (:then_1
      (bind _jumpdirection_2 (Timeline|Timeline_0 PlayFromStart)
        (:Update
          (Transformation|AddLocalOffset _mesh _jumpdirection_2 false false))
        (:Finished
          (Utilities|FlowControl|Delay 1.0)
          (Transformation|SetRelativeLocation _mesh "0, 0,-90.000000" false false))))))

(event EventBeginPlay
  (|CallParentFunction)
  ;[1 1 1] Bind Event On see
  (EventDispatchers|AssignOnSeePawn (Variables|Default|GetPawnSensing) (delegate Custom|OnSeePawn_Event_0)))

(event Collision|EventActorBeginOverlap
  (params (OtherActor :type Actor%20Object%20Reference))
  (|CallParentFunction OtherActor) ; This node is disabled and will not be called.\nDrag off pins to build functionality.
)

(event EventTick
  (params (DeltaSeconds :type Float%20%28single-precision%29))
  (|CallParentFunction DeltaSeconds)
  (Utilities|FlowControl|Sequence
    (:then_0
      ;[1 1 1] Get velocity
      (Variables|Default|SetSpeed (Math|Vector|VectorLength (Transformation|GetVelocity self))))
    (:then_1
      ;[1 1 1] Set distance With player
      (Variables|Default|SetDistanceWithPlayer (Math|Vector|Distance(Vector) (Transformation|GetActorLocation self) (Transformation|GetActorLocation (Game|Player|GetPlayerPawn 0)))))
    (:then_2
      (if (Math|Boolean|ANDBoolean (< (Variables|Default|GetDistanceWithPlayer) (Variables|Default|GetJumpAttackRange)) (Variables|Default|GetJumpAvailable) (Variables|Default|GetInFight?))
        (Utilities|FlowControl|DoOnce false
          (:Completed
            (Variables|Default|SetJumpAttackStart true)
            (CallFunction|JumpAttack)))))))

(fn ConstructionScript
  (|CallParentFunction)
  (Variables|Default|SetInFight? false)
  (Variables|/Script/Engine.CharacterMovementComponent|SetMaxWalkSpeed (Variables|Character|GetCharacterMovement) (Variables|Default|GetPatrolSpeed)))