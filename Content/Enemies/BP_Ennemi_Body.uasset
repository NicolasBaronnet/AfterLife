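; Enemy character body with melee, projectile, fly-away, hit-reaction and stun actions, exposed as events and functions.
; At zero HP it enters timed stasis with execution prompts that react to player distance, reviving at full health unless killed.
; Execution or Banishement ragdolls it and notifies the game mode.
; Devouring moves it to another enemy and destroys that target, boosting health, damage, speed and animation rate, with material and scale stages.
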(event Custom|Stasis%20event
  ;[1 1 1] Stasis Gesture
  (Utilities|FlowControl|DoOnce false
    (:Completed
      (Animation|StopAnimMontage (Animation|GetCurrentMontage :!class /Script/Engine.Character))
      (Variables|State|SetOccupied true)
      (Variables|State|SetInStasis true)
      (bind _returnvalue (Utilities|Time|SetTimerbyEvent (delegate Custom|Stase%20Timing) 1.0 true))
      (Variables|Stase|SetTimerStase _returnvalue)
      (Rendering|Material|SetMaterial (Variables|Character|GetMesh) 0 (Variables|System|GetStasisMaterial))
      (Rendering|SetVisibility (Variables|Default|GetButtonE) true false)
      (Rendering|SetVisibility (Variables|Default|GetButtonA) true false))))

(event Custom|Attack%20Mélée%20%20Event
  ;[1 1 1] Attack Animation
  (Variables|State|SetOccupied true)
  (bind _notifyname (Animation|Montage|PlayMontage (Variables|Character|GetMesh) "/Game/Enemies/01_Starved/Animations/Montages/Boss_Attack_Swing_InP_Montage.Boss_Attack_Swing_InP_Montage" (Variables|Statistics|GetAnimationPlayRate))
    (:then
      (CallFunction|DamagetoApply (Variables|Statistics|GetDamageInput) 1.0))
    (:OnCompleted
      (Variables|State|SetOccupied false)
      (Variables|State|SetCantBeCancel? false))
    (:OnNotifyBegin
      (switch name _notifyname
        (:Recovery
          (Variables|State|SetCantBeCancel? false))
        (:CantBeCancel
          (Variables|State|SetCantBeCancel? true))))))

(event Custom|Range%20Attack
  ;[1 1 1] Range Attack
  (Variables|State|SetOccupied false)
  (bind _notifyname (Animation|Montage|PlayMontage (Variables|Character|GetMesh) "/Game/Enemies/01_Starved/Animations/Montages/Boss_Staggered_InP_Montage.Boss_Staggered_InP_Montage" (Variables|Statistics|GetAnimationPlayRate))
    (:OnCompleted
      _)
    (:OnInterrupted
      _)
    (:OnNotifyBegin
      (switch name _notifyname
        (:Hit
          (Game|SpawnActorfromClass "/Game/Enemies/02_Errinye/BP_Projectile.BP_Projectile_C" (Transformation|GetWorldTransform (Variables|Default|GetArrow1)) "Undefined" self 0)))))
  (Variables|State|SetOccupied true))

(event Custom|Stase%20Timing
  ;[1 1 1] Stasis Gesture
  (if (not (Variables|State|GetDead))
    (Math|Integer|IncrementInt (Variables|Stase|GetStaseTimer)
      (:%20%20
        (if (>= (Variables|Stase|GetStaseTimer) (Variables|Stase|GetStaseDuration))
          (Utilities|Time|ClearandInvalidateTimerbyHandle (Variables|Stase|GetTimerStase))
          (Variables|Stase|SetStaseTimer 0)
          (bind _output_get (Variables|Statistics|SetActualHP (Variables|Statistics|GetMaxHp)))
          (Variables|/Game/Enemies/01_Starved/UI/UI_Hp_Starved.UI_Hp_Starved_C|SetActualHP_Ref (Variables|System|GetHpUiRef) _output_get)
          (Rendering|Material|SetMaterial (Variables|Character|GetMesh) 0 (Variables|System|GetBaseMaterial))
          (Variables|State|SetDead false)
          (Variables|State|SetOccupied false)
          (Variables|State|SetInStasis false)
          (Rendering|SetVisibility (Variables|Default|GetButtonE) false false)
          (Rendering|SetVisibility (Variables|Default|GetButtonA) false false)
          (Utilities|FlowControl|DoOnce false) ; enters at Reset
        )))
    (else
      (Utilities|Time|ClearandInvalidateTimerbyHandle (Variables|Stase|GetTimerStase)))))

(event Custom|FlyAway
  (bind _returnvalue (Game|Player|GetPlayerPawn 0))
  (bind _self self)
  (bind _charactermovement (Variables|Character|GetCharacterMovement))
  (bind _returnvalue_2 (Pawn|GetNavAgentLocation _self))
  (bind _returnvalue_3 (Transformation|GetActorLocation _returnvalue))
  (bind _returnvalue_4 (Math|Vector|GetUnitDirection(Vector) _returnvalue_3 _returnvalue_2))
  (bind _returnvalue_5 (Math|Vector|MakeVector (.x _returnvalue_4) (.y _returnvalue_4) 0.0))
  ;[1 1 1] Fly Away
  (Utilities|FlowControl|DoOnce false :!label _label
    (:Completed
      (Variables|Fly|SetCanFly false)
      (Utilities|FlowControl|Sequence
        (:then_0
          (Utilities|FlowControl|Delay (Variables|Fly|GetFly%20Cool%20Down))
          (Variables|Fly|SetCanFly true)
          (goto _label Reset))
        (:then_1
          (Character|Jump)
          (Variables|/Script/Engine.CharacterMovementComponent|SetMaxWalkSpeed _charactermovement (Variables|Fly|GetFlying%20Speed))
          (Timeline|Timeline_0 PlayFromStart
            (:Update
              (Pawn|Input|AddMovementInput (Math|Vector|MakeVector (.x _returnvalue_5) (.y _returnvalue_5) 0.0) 1.0 false))
            (:Finished
              (Variables|/Script/Engine.CharacterMovementComponent|SetMaxWalkSpeed _charactermovement (Variables|Statistics|GetDefault%20Walk%20Speed)))))))))

(event Custom|Devour%20Event
  (params (Ennemie%20to%20devour :type BP%20Ennemi%20Body%20Object%20Reference))
  ;[1 1 1] Fonction de dévorer
  (Utilities|FlowControl|DoOnce false :!label _label
    (:Completed
      (Animation|StopAnimMontage (Animation|GetCurrentMontage :!class /Script/Engine.Character))
      (Variables|Default|SetbCanBeDamaged false)
      (Variables|State|SetOccupied true)
      (Variables|Devour|SetIsDevour? true)
      (AI|AIMoveTo self "0, 0, 0" Ennemie%20to%20devour 8e+01 false
        (:OnSuccess
          (Animation|Montage|PlayMontage (Variables|Character|GetMesh) "/Game/Enemies/01_Starved/Animations/Montages/Boss_Attack_HandAndSwordSwing_InP_Montage.Boss_Attack_HandAndSwordSwing_InP_Montage" 1.5
            (:OnCompleted
              (Utilities|IsValid Ennemie%20to%20devour :!label _label_2
                (:Is%20Valid
                  (Actor|DestroyActor Ennemie%20to%20devour)
                  (CallFunction|DevourSatsGesture))
                (:Is%20Not%20Valid
                  _))
              (Variables|State|SetOccupied false)
              (Variables|Default|SetbCanBeDamaged true)
              (Variables|Devour|SetIsDevour? false)
              (goto _label Reset))
            (:OnBlendOut
              (goto _label_2))
            (:OnInterrupted
              _)))
        (:OnFail
          (Development|PrintString "Fail to reach corps")))
      (Variables|State|SetOccupied false)
      (Variables|Default|SetbCanBeDamaged true)
      (Variables|Devour|SetIsDevour? false))))

(event Custom|Stun%20Event
  (params (Bump%20direction :type Vector))
  ;[1 1 1] Stun gesture
  (Utilities|FlowControl|Sequence
    (:then_0
      ;;[1 1 1] Stun Gesture
      (Utilities|FlowControl|DoOnce false
        (:Completed
          (bind _returnvalue (Utilities|Time|SetTimerbyEvent (delegate Custom|Stun%20event%20Timer) 0.1 true))
          (Variables|Default|SetStunTimerHandle _returnvalue)
          (Animation|Montage|PlayMontage (Variables|Character|GetMesh) "/Game/Enemies/01_Starved/Animations/Montages/Boss_Staggered_InP_Montage.Boss_Staggered_InP_Montage"
            (:then
              (Audio|PlaySound2D "/Game/Sounds/Cue/SC_ShieldBlock.SC_ShieldBlock" 1.0 1.0 0.0 0 0)
              (bind _returnvalue_2 (Effects|SpawnEmitteratLocation "/Game/Plugs_In/Particles/P_Sparks.P_Sparks" (Transformation|GetWorldLocation (Variables|Default|GetSparkSpawn))))
              (Utilities|FlowControl|Delay 0.2)
              (Components|DestroyComponent _returnvalue_2))))))
    (:then_1
      (Transformation|AddActorWorldOffset (* Bump%20direction -1e+01)))))

(event Custom|Stun%20event%20Timer
  ;[1 1 1] Stun gesture
  ;;[1 1 1] Stun Gesture
  (if (<= (Variables|Default|GetStunCount) (Variables|Default|GetStunDuration))
    (Variables|State|SetIsStunned? true)
    (Rendering|SetVisibility (Variables|Default|GetStunIndicator) true false)
    (Math|Integer|IncrementInt (Variables|Default|GetStunCount))
    (else
      (Utilities|Time|ClearandInvalidateTimerbyHandle (Variables|Default|GetStunTimerHandle))
      (Variables|Default|SetStunCount 0)
      (Variables|State|SetIsStunned? false)
      (Rendering|SetVisibility (Variables|Default|GetStunIndicator) false false)
      (Utilities|FlowControl|DoOnce false) ; enters at Reset
    )))

(event EventBeginPlay
  ;[1 1 1] Begin Play
  (Utilities|FlowControl|Sequence
    (:then_0
      ;;[1 1 1] Get ref player
      (bind _asbp_hero (Utilities|Casting|CastToBP_Hero (Game|Player|GetPlayerPawn 0)))
      (Variables|System|SetPlayerRef _asbp_hero))
    (:then_1
      ;;[1 1 1] Begin play set up
      (bind _asui_hp_starved (Utilities|Casting|CastToUI_Hp_Starved (UserInterface|GetUserWidgetObject (Variables|Default|GetHealthBar))))
      (Variables|System|SetHpUiRef _asui_hp_starved))
    (:then_2
      (Variables|/Game/Enemies/01_Starved/UI/UI_Hp_Starved.UI_Hp_Starved_C|SetActualHP_Ref (Variables|System|GetHpUiRef) (Variables|Statistics|GetActualHP))
      (Variables|/Game/Enemies/01_Starved/UI/UI_Hp_Starved.UI_Hp_Starved_C|SetMaxHpRef (Variables|System|GetHpUiRef) (Variables|Statistics|GetMaxHp)))))

(event EventTick
  (params (DeltaSeconds :type Float%20%28single-precision%29))
  (bind _button_rotation (Variables|Stase|GetButton%20Rotation))
  (bind _playerref (Variables|System|GetPlayerRef))
  (bind _returnvalue (Transformation|GetDistanceTo _playerref))
  ;[1 1 1] Execution Button Gesture
  (Utilities|FlowControl|Sequence
    (:then_0
      (Transformation|AddRelativeRotation (Variables|Default|GetButtonA) (Math|Rotator|MakeRotator _button_rotation 0.0 0.0) false false)
      (Transformation|AddRelativeRotation (Variables|Default|GetButtonE) (Math|Rotator|MakeRotator _button_rotation 0.0 0.0) false false))
    (:then_1
      (Variables|Execution|SetDistanceToPlayer _returnvalue)
      (if (< _returnvalue (Variables|/Game/Hero/BP_Hero.BP_Hero_C|GetExecutionDistance _playerref))
        (Utilities|FlowControl|DoOnce false :!label _label
          (:Completed
            (Rendering|Material|SetMaterial (Variables|Default|GetButtonE) 0 "/Game/Materials/Blocking_MAterials/M_Green.M_Green")
            (Rendering|Material|SetMaterial (Variables|Default|GetButtonA) 0 "/Game/Materials/Blocking_MAterials/M_Green.M_Green")
            (goto _label_2 Reset)))
        (else
          (Utilities|FlowControl|DoOnce false :!label _label_2
            (:Completed
              (Rendering|Material|SetMaterial (Variables|Default|GetButtonE) 0 "/Game/Materials/Blocking_MAterials/M_floor.M_floor")
              (Rendering|Material|SetMaterial (Variables|Default|GetButtonA) 0 "/Game/Materials/Blocking_MAterials/M_floor.M_floor")
              (goto _label Reset))))))
    (:then_2
      (Utilities|FlowControl|DoOnce false :!label _label_3
        (:Completed
          (bind _movementvalue (Timeline|Stun%20Indicator%20movement PlayFromStart)
            (:Update
              (Transformation|AddRelativeLocation (Variables|Default|GetStunIndicator) (Math|Vector|MakeVector 0.0 0.0 _movementvalue) false false))
            (:Finished
              (goto _label_3 Reset))))))))

(event Game|Damage|EventAnyDamage
  (params (Damage :type Float%20%28single-precision%29) (DamageType :type Damage%20Type%20Object%20Reference) (InstigatedBy :type Controller%20Object%20Reference) (DamageCauser :type Actor%20Object%20Reference))
  ;[1 1 1] Event take dammage
  (if (Variables|Default|GetbCanBeDamaged)
    (Utilities|Casting|CastToBP_Hero DamageCauser)
    (Utilities|FlowControl|Sequence
      (:then_0
        (Variables|Default|SetbCanBeDamaged false)
        (Variables|State|SetOccupied true)
        (CallFunction|LifeGestureFunction Damage))
      (:then_1
        (if (Variables|State|GetCantBeCancel?)
          (Utilities|FlowControl|Delay 0.25)
          (else
            (Animation|StopAnimMontage (Animation|GetCurrentMontage :!class /Script/Engine.Character))
            (bind _notifyname (Animation|Montage|PlayMontage (Variables|Character|GetMesh) "/Game/Enemies/01_Starved/Animations/Montages/Boss_ReactionHit_R_Montage.Boss_ReactionHit_R_Montage")
              (:OnCompleted
                _)
              (:OnInterrupted
                _)
              (:OnNotifyBegin
                (switch name _notifyname
                  (:Recovery
                    _))))))
        (Variables|Default|SetbCanBeDamaged true)
        (Variables|State|SetOccupied false))
      (:then_2
        (Audio|PlaySoundatLocation "/Game/Sounds/Cue/SC_DashImpact.SC_DashImpact" (Transformation|GetActorLocation self) "0, 0, 0" 1.0 1.0 0.0 0 0 0)))))

(fn ConstructionScript
  (Utilities|FlowControl|Sequence
    (:then_0
      (Variables|Statistics|SetActualHP (Variables|Statistics|GetMaxHp))
      (Variables|/Script/Engine.CharacterMovementComponent|SetMaxWalkSpeed (Variables|Character|GetCharacterMovement) (Variables|Statistics|GetDefault%20Walk%20Speed)))
    (:then_1
      (Rendering|SetVisibility (Variables|Default|GetButtonE) false false)
      (Rendering|SetVisibility (Variables|Default|GetButtonA) false false)
      (Rendering|Material|SetMaterial (Variables|Character|GetMesh) 0 (Utilities|Array|Get(acopy) (Variables|Devour|GetMaterialChangOnDevour)))
      (Rendering|SetVisibility (Variables|Default|GetStunIndicator) false false))))

(fn LifeGestureFunction
  (params (DamageInput :type Float%20%28single-precision%29))
  (bind _output_get (Variables|Statistics|SetActualHP (- (Variables|Statistics|GetActualHP) DamageInput)))
  (if (< _output_get 0.0)
    (Variables|Statistics|SetActualHP 0.0)
    (CallFunction|StasisEvent))
  (Variables|/Game/Enemies/01_Starved/UI/UI_Hp_Starved.UI_Hp_Starved_C|SetActualHP_Ref (Variables|System|GetHpUiRef) (Variables|Statistics|GetActualHP)))

(fn DeathFunction
  (bind _returnvalue (Utilities|Name|MakeLiteralName "pelvis"))
  (bind _mesh (Variables|Character|GetMesh))
  (Animation|StopAnimMontage (Animation|GetCurrentMontage :!class /Script/Engine.Character))
  (Collision|SetCollisionProfileName (Variables|Character|GetMesh) "IgnoreOnlyPawn" true :!class /Script/Engine.PrimitiveComponent)
  (Collision|SetCollisionEnabled (Variables|Character|GetMesh) "QueryAndPhysics")
  (Class|SkeletalMeshComponent|SetAllBodiesBelowSimulatePhysics (Variables|Character|GetMesh) _returnvalue true true)
  (Class|SkeletalMeshComponent|SetAllBodiesBelowPhysicsBlendWeight (Variables|Character|GetMesh) _returnvalue 1.0 false true)
  (Collision|SetCollisionEnabled (Variables|Default|GetCapsuleComponent) "NoCollision")
  (Rendering|SetVisibility (Variables|Default|GetHealthBar) false false)
  (Collision|SetCollisionProfileName _mesh "Custom" true :!class /Script/Engine.PrimitiveComponent)
  (Collision|SetCollisionObjectType _mesh "ECC_GameTraceChannel3")
  (Rendering|SetVisibility (Variables|Default|GetButtonE) false false)
  (Rendering|SetVisibility (Variables|Default|GetButtonA) false false)
  (Variables|State|SetDead true)
  (Default|CallEDEnnemiDeath (CallFunction|GetGameMod)))

(fn DamagetoApply
  (params (DamageInput :type Float%20%28single-precision%29) (Multiplier :type Float%20%28single-precision%29))
  (Variables|Fight|SetDamagesToApply (* DamageInput Multiplier)))

(fn CastDamagetoTarget
  (bind (_outhits _returnvalue) (Class|KismetSystemLibrary|BoxTraceMultiforObjects (Transformation|GetSocketLocation (Variables|Character|GetMesh) "TrailBotSocket") (Transformation|GetSocketLocation (Variables|Character|GetMesh) "TrailTopSocket") "50.000000,50.000000,50.000000" (Transformation|GetWorldRotation (Variables|Default|GetGreatAxe)) (Utilities|Array|MakeArray "ObjectTypeQuery8" "ObjectTypeQuery6") false 0 "None" true))
  (if _returnvalue
    (for _array_element _outhits
      (bind _asbp_destructible (Utilities|Casting|CastToBP_Destructible (.HitActor (Collision|BreakHitResult _array_element)))
        (:then
          (Default|SetImpulsePointDamage _asbp_destructible (.ImpactPoint (Collision|BreakHitResult _array_element)) (.ImpactNormal (Collision|BreakHitResult _array_element))))
        (:CastFailed
          _))
      (Game|Damage|ApplyDamage (.HitActor (Collision|BreakHitResult _array_element)) (Variables|Fight|GetDamagesToApply) 0 self))))

(fn Banishement
  (CallFunction|DeathFunction)
  (|CallParentFunction))

(fn Execution
  (CallFunction|DeathFunction)
  (|CallParentFunction))

(fn DevourSatsGesture
  (bind _hpuiref (Variables|System|GetHpUiRef))
  (Variables|Statistics|SetMaxHp (* (Variables|Statistics|GetMaxHp) (Variables|Statistics|GetDevourStatsIncresement)))
  (Variables|Statistics|SetActualHP (Variables|Statistics|GetMaxHp))
  (Variables|Statistics|SetDamageInput (* (Variables|Statistics|GetDamageInput) (Variables|Statistics|GetDevourStatsIncresement)))
  (Variables|/Game/Enemies/01_Starved/UI/UI_Hp_Starved.UI_Hp_Starved_C|SetMaxHpRef _hpuiref (Variables|Statistics|GetMaxHp))
  (Variables|/Game/Enemies/01_Starved/UI/UI_Hp_Starved.UI_Hp_Starved_C|SetActualHP_Ref _hpuiref (Variables|Statistics|GetActualHP))
  (Variables|/Script/Engine.CharacterMovementComponent|SetMaxWalkSpeed (Variables|Character|GetCharacterMovement) (* (Variables|Statistics|GetDefault%20Walk%20Speed) (Variables|Statistics|GetDevourStatsIncresement)))
  (Variables|Statistics|SetAnimationPlayRate (* (* (Variables|Statistics|GetAnimationPlayRate) (Variables|Statistics|GetDevourStatsIncresement)) 0.9))
  (if (< (Variables|Devour|GetDevourNumberOfState) (- (Utilities|Array|Length (Variables|Devour|GetMaterialChangOnDevour)) 1))
    (bind _result (Math|Integer|IncrementInt (Variables|Devour|GetDevourNumberOfState))
      (:%20%20
        (Rendering|Material|SetMaterial (Variables|Character|GetMesh) 0 (Utilities|Array|Get(acopy) (Variables|Devour|GetMaterialChangOnDevour) _result))
        (Transformation|SetActorScale3D self (* (Transformation|GetWorldScale (Variables|Default|GetCapsuleComponent)) (* (Variables|Statistics|GetDevourStatsIncresement) 0.9)))))))