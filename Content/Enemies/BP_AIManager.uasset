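; BP_AIManager is an enemy AI manager actor that keeps a shared ticket count adjusted through game mode event dispatchers.
; The ask-ticket handler decrements TicketNumber and the refund-ticket handler increments it, with no limit check.
; On BeginPlay it binds the refund handler to the game mode's dispatcher but unbinds, rather than binds, the ask handler, so this graph never subscribes to ticket requests.
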(event Custom|ED%20Ask%20Ticket
  (Variables|Default|SetTicketNumber (- (Variables|Default|GetTicketNumber) 1)))

(event Custom|ED%20Refund%20Ticket
  (Variables|Default|SetTicketNumber (+ (Variables|Default|GetTicketNumber) 1)))

(event EventBeginPlay
  (bind _gamemodref (CallFunction|GetGameMod))
  (Utilities|FlowControl|Sequence
    (:then_0
      (EventDispatchers|UnbindEventfromEDAskTicket _gamemodref (delegate Custom|ED%20Ask%20Ticket)))
    (:then_1
      (EventDispatchers|BindEventtoEDRefundTicket _gamemodref (delegate Custom|ED%20Refund%20Ticket)))))

(event Collision|EventActorBeginOverlap
  (params (OtherActor :type Actor%20Object%20Reference)))

(event EventTick
  (params (DeltaSeconds :type Float%20%28single-precision%29)))

(fn ConstructionScript)