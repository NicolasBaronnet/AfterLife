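; Homing projectile for the Errinye enemy that damages the hero and destructible objects.
; On BeginPlay it homes on the player pawn's root component and destroys itself after its lifetime.
; Box overlaps ignore enemy bodies, damage the hero, or set an impact impulse point on destructibles before damaging them.
; Any other overlap, or any box hit, destroys the projectile.
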(event OnComponentHit(Box)
  (params (HitComponent :type Primitive%20Component%20Object%20Reference) (OtherActor :type Actor%20Object%20Reference) (OtherComp :type Primitive%20Component%20Object%20Reference) (NormalImpulse :type Vector :default "0, 0, 0") (Hit :type Hit%20Result%20Structure%20%28by%20ref%29))
  (Actor|DestroyActor))

(event OnComponentBeginOverlap(Box)
  (params (OverlappedComponent :type Primitive%20Component%20Object%20Reference) (OtherActor :type Actor%20Object%20Reference) (OtherComp :type Primitive%20Component%20Object%20Reference) (OtherBodyIndex :type Integer) (bFromSweep :type Boolean) (SweepResult :type Hit%20Result%20Structure%20%28by%20ref%29))
  (bind (_bblockinghit _binitialoverlap _time _distance _location _impactpoint _normal _impactnormal _physmat _hitactor) (Collision|BreakHitResult SweepResult))
  (Utilities|Casting|CastToBP_Ennemi_Body OtherActor
    (:CastFailed
      (bind _asbp_hero (Utilities|Casting|CastToBP_Hero OtherActor)
        (:then
          (Game|Damage|ApplyDamage _asbp_hero (Variables|Default|GetErrinyeDamages) 0 self)
          (Actor|DestroyActor))
        (:CastFailed
          (bind _asbp_destructible (Utilities|Casting|CastToBP_Destructible OtherActor)
            (:then
              (Default|SetImpulsePointDamage _asbp_destructible _impactpoint _impactnormal)
              (Game|Damage|ApplyDamage _hitactor (Variables|Default|GetErrinyeDamages) 0 self)
              (Actor|DestroyActor))
            (:CastFailed
              (Actor|DestroyActor))))))))

(event EventBeginPlay
  (Variables|/Script/Engine.ProjectileMovementComponent|SetHomingTargetComponent (Variables|Default|GetProjectileMovement) (Variables|/Script/Engine.Actor|GetRootComponent (Game|Player|GetPlayerPawn 0)))
  (Utilities|FlowControl|Delay (Variables|Default|GetLifeTime))
  (Actor|DestroyActor))

(fn ConstructionScript)