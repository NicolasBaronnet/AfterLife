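; BP_SoundManager is a sound manager actor that runs wind, music and ambient audio layers, starting them on BeginPlay.
; ChangeWind, ChangeMusic and NewAmbiance each swap one layer's sound via fade out, delay and fade in, sharing FadeDuration.
; An inspection handler uses a FlipFlop to toggle muffled, low-pitched wind and ambience with an inspection loop, but its dispatcher binding is never executed.
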(event Custom|ED_Inspection_Event_0
  (bind _windsound (Variables|Default|GetWindSound))
  (bind _music (Variables|Default|GetMusic))
  (Utilities|FlowControl|FlipFlop
    (:A
      (Audio|Components|Audio|SetPitchMultiplier _windsound 0.2)
      (Audio|Components|Audio|SetVolumeMultiplier _windsound 0.4 :!class /Script/Engine.AudioComponent)
      (Audio|Components|Audio|SetVolumeMultiplier _music 0.8 :!class /Script/Engine.AudioComponent)
      (Audio|Components|Audio|Play (Variables|Default|GetInspectingLoop) 0.0))
    (:B
      (Audio|Components|Audio|SetPitchMultiplier _windsound 1.0)
      (Audio|Components|Audio|SetVolumeMultiplier _windsound 1.0 :!class /Script/Engine.AudioComponent)
      (Audio|Components|Audio|SetVolumeMultiplier _music 0.8 :!class /Script/Engine.AudioComponent)
      (Audio|Components|Audio|Stop (Variables|Default|GetInspectingLoop)))))

(event Custom|ChangeWind
  (params (NewWind :type Sound%20Cue%20Object%20Reference))
  (Audio|Components|Audio|FadeOut (Variables|Default|GetWindSound) (Variables|Default|GetFadeDuration) 0.0 "Linear" :!class /Script/Engine.AudioComponent)
  (Utilities|FlowControl|Delay (Variables|Default|GetFadeDuration))
  (Audio|Components|Audio|SetSound (Variables|Default|GetWindSound) NewWind)
  (Audio|Components|Audio|FadeIn (Variables|Default|GetWindSound) (Variables|Default|GetFadeDuration) 1.0 0.0 "Linear" :!class /Script/Engine.AudioComponent))

(event Custom|Change%20Music
  (params (New%20Music :type Sound%20Cue%20Object%20Reference))
  (Audio|Components|Audio|FadeOut (Variables|Default|GetMusic) (Variables|Default|GetFadeDuration) 0.0 "Linear" :!class /Script/Engine.AudioComponent)
  (Utilities|FlowControl|Delay (Variables|Default|GetFadeDuration))
  (Audio|Components|Audio|SetSound (Variables|Default|GetMusic) New%20Music)
  (Audio|Components|Audio|FadeIn (Variables|Default|GetMusic) (Variables|Default|GetFadeDuration) 1.0 0.0 "Linear" :!class /Script/Engine.AudioComponent))

(event Custom|New%20Ambiance
  (params (New%20Ambiance :type Sound%20Cue%20Object%20Reference))
  (Audio|Components|Audio|FadeOut (Variables|Default|GetAmbiantSound) (Variables|Default|GetFadeDuration) 0.0 "Linear" :!class /Script/Engine.AudioComponent)
  (Utilities|FlowControl|Delay (Variables|Default|GetFadeDuration))
  (Audio|Components|Audio|SetSound (Variables|Default|GetAmbiantSound) New%20Ambiance)
  (Audio|Components|Audio|FadeIn (Variables|Default|GetAmbiantSound) (Variables|Default|GetFadeDuration) 1.0 0.0 "Linear" :!class /Script/Engine.AudioComponent))

(event EventBeginPlay
  (Audio|Components|Audio|Play (Variables|Default|GetWindSound) 0.0)
  (Audio|Components|Audio|Stop (Variables|Default|GetInspectingLoop)))

(event Collision|EventActorBeginOverlap
  (params (OtherActor :type Actor%20Object%20Reference)))

(event EventTick
  (params (DeltaSeconds :type Float%20%28single-precision%29)))

(fn ConstructionScript)