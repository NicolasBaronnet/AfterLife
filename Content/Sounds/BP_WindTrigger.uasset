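; BP_WindTrigger is a trigger volume that switches the wind and ambient sounds when the hero enters it.
; On box overlap by BP_Hero, it compares the names of the sound manager's current sounds with its NewWind and NewAmbiance sounds.
; It asks the referenced sound manager to change only those that differ, and the ambiance only if NewAmbiance is valid.
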(event OnComponentBeginOverlap(Box)
  (params (OverlappedComponent :type Primitive%20Component%20Object%20Reference) (OtherActor :type Actor%20Object%20Reference) (OtherComp :type Primitive%20Component%20Object%20Reference) (OtherBodyIndex :type Integer) (bFromSweep :type Boolean) (SweepResult :type Hit%20Result%20Structure%20%28by%20ref%29))
  (bind _new_ambiance (Variables|Default|GetNew%20Ambiance))
  (bind _soundmanagerref (Variables|Default|GetSoundManagerRef))
  (Utilities|Casting|CastToBP_Hero OtherActor)
  (if (Utilities|Enum|Equal(Enum) (Utilities|GetObjectName (Variables|/Script/Engine.AudioComponent|GetSound (Variables|/Game/Sounds/BP_SoundManager.BP_SoundManager_C|GetWindSound (Variables|Default|GetSoundManagerRef)))) (Utilities|GetObjectName (Variables|Default|GetNewWind)))
    _
    (else
      (Default|ChangeWind _soundmanagerref (Variables|Default|GetNewWind))))
  (if (and (Utilities|IsValid _new_ambiance) (not (Utilities|Enum|Equal(Enum) (Utilities|GetObjectName (Variables|/Script/Engine.AudioComponent|GetSound (Variables|/Game/Sounds/BP_SoundManager.BP_SoundManager_C|GetAmbiantSound (Variables|Default|GetSoundManagerRef)))) (Utilities|GetObjectName (Variables|Default|GetNew%20Ambiance)))))
    (Default|NewAmbiance _soundmanagerref _new_ambiance)))

(event EventBeginPlay)

(event Collision|EventActorBeginOverlap
  (params (OtherActor :type Actor%20Object%20Reference)))

(event EventTick
  (params (DeltaSeconds :type Float%20%28single-precision%29)))

(fn ConstructionScript)